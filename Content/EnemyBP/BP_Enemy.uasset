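; Enemy that patrols between its spawn point and a Goal offset, chases the player on sight and opens MainMap once within catching range.
; Each Tick sweeps a fan of line traces across its view angle; a Player-tagged hit latches IsPaused, driving SimpleMoveToActor until the player exceeds MaxDistance.
; Patrol timers pause during the chase.
; A camera-facing widget shows while the player is detected.
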(event `self.ReceiveTick`
  (params (DeltaSeconds :type "Float (single-precision)"))
  (bind _widget (`self.Widget`))
  (bind _ishit (`self.isHit`))
  (bind _last_index (`self.Last Index`))
  (bind _widget_2 (`self.Widget`))
  (bind _returnvalue (+ (`self.K2_GetActorLocation`) (0.0 0.0 65.0)))
  (`SceneComponent.K2_SetWorldRotation` _widget (`KismetMathLibrary.MakeRotator` (.roll (`SceneComponent.K2_GetComponentRotation` _widget)) (.pitch (`SceneComponent.K2_GetComponentRotation` _widget)) (.yaw (`KismetMathLibrary.FindLookAtRotation` (`SceneComponent.K2_GetComponentLocation` _widget) (`PlayerCameraManager.GetCameraLocation` (`GameplayStatics.GetPlayerCameraManager` 0))))) false false)
  (`KismetArrayLibrary.Array_Resize` (`self.isHit`) (`self.Last Index`))
  (for _index (range (+ (`self.Last Index`) 1))
    (set `self.CurrentAngle` (- (* _index (`self.SpacingAngle`)) (`self.Angle`)))
    (if (or (`self.isVisibility`) (`self.isPaused`))
      (`self.MoveToPlayer`))
    (bind (_outhit _returnvalue_2) (`KismetSystemLibrary.LineTraceSingle` :`Start` _returnvalue :`End` (+ _returnvalue (* (`KismetMathLibrary.RotateAngleAxis` (`self.GetActorForwardVector`) (`self.CurrentAngle`) (0.0 0.0 1.0)) (`self.Distance`))) :`TraceChannel` "TraceTypeQuery2" :`DrawDebugType` "ForDuration" :`DrawTime` 0.0))
    (`self.MoveTimer`)
    (if _returnvalue_2
      (if (`self.ActorHasTag` (`.HitActor` (`GameplayStatics.BreakHitResult` _outhit)) "Player")
        (set `self.isPaused` true)
        (`KismetArrayLibrary.Array_Insert` _ishit true _last_index)
        (else
          (`KismetArrayLibrary.Array_Insert` _ishit false _last_index :!label _label)))
      (else
        (goto _label))))
  (for _array_element (`self.isHit`)
    (if _array_element
      (set `self.isVisibility` true) ; 一つでもhitしていればTrue
    ))
  (if (`self.isVisibility`)
    (`SceneComponent.SetVisibility` _widget_2 true false)
    (set `self.isVisibility` false)
    (else
      (`SceneComponent.SetVisibility` _widget_2 false false)
      (`self.MoveTimer`))))

(event `MoveToPlayer`
  (bind _returnvalue (`GameplayStatics.GetPlayerPawn` 0))
  (bind _returnvalue_2 (`self.GetHorizontalDistanceTo` _returnvalue))
  (`AIBlueprintHelperLibrary.SimpleMoveToActor` (`AIBlueprintHelperLibrary.GetAIController` self) _returnvalue)
  (if (> 100.0 _returnvalue_2)
    (`GameplayStatics.OpenLevel` "MainMap")
    (elif (> _returnvalue_2 (`self.maxDistance`))
      (set `self.isPaused` false)
      (`self.MoveTimer`))))

(event `self.ReceiveBeginPlay`
  (bind _output_get (set `self.Last Index` (`KismetMathLibrary.FCeil` (/ (* (`self.Angle`) 2.0) (`self.SpacingAngle`)))))
  (set `self.SpacingAngle` (/ (* (`self.Angle`) 2.0) (`KismetMathLibrary.Conv_IntToDouble` _output_get)))
  (set `self.Default_location` (`self.K2_GetActorLocation`))
  (`AIBlueprintHelperLibrary.SimpleMoveToLocation` (`AIBlueprintHelperLibrary.GetAIController` self) (+ (`self.Goal`) (`self.K2_GetActorLocation` self)))
  (`self.NormalMove`)
  (bind _returnvalue (`KismetSystemLibrary.K2_SetTimerDelegate` (delegate `MoveDefault`) 7.0 true)))

(event `MoveDefault`
  (`AIBlueprintHelperLibrary.SimpleMoveToLocation` (`AIBlueprintHelperLibrary.GetAIController` self) (`self.Default_location`))
  (bind _returnvalue (`KismetSystemLibrary.K2_SetTimerDelegate` (delegate `MoveToGoal`) 3.0)))

(event `MoveTimer`
  (bind _returnvalue (or (`self.isVisibility`) (`self.isPaused`)))
  (if _returnvalue
    (`KismetSystemLibrary.K2_PauseTimerHandle` (stale `self.ReceiveBeginPlay` _returnvalue))
    (else
      (`KismetSystemLibrary.K2_UnPauseTimerHandle` (stale `self.ReceiveBeginPlay` _returnvalue))))
  (if _returnvalue
    (`KismetSystemLibrary.K2_PauseTimerHandle` (stale `MoveDefault` _returnvalue))
    (else
      (`KismetSystemLibrary.K2_UnPauseTimerHandle` (stale `MoveDefault` _returnvalue)))))

(event `MoveToGoal`
  (`AIBlueprintHelperLibrary.SimpleMoveToLocation` (`AIBlueprintHelperLibrary.GetAIController` self) (+ (`self.Goal`) (`self.K2_GetActorLocation` self))))

(fn `GetIsPaused`
  (returns (isPaused :type Boolean))
  (return (`self.isPaused`)))

(fn `NormalMove`
  (`KismetSystemLibrary.K2_SetTimerDelegate` (`|CreateDelegate` :!event `MoveTimer`) 7.0 true))

(event `MoveToDefault`
  (`AIBlueprintHelperLibrary.SimpleMoveToLocation` (`AIBlueprintHelperLibrary.GetAIController` self) (`self.Default_location`)))

(fn `UserConstructionScript`)